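; Projectile actor for the Infinite Matrix game that ties its movement speed settings to the player's forward speed.
; BeginPlay caches the BP_Player pawn, and Tick rewrites the ProjectileMovement initial and max speeds as multiples of that speed.
; A lifetime counter adds delta time and compounds by a multiplier every tick, so the projectile destroys itself at a frame-rate-dependent time before three real seconds pass.
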(event EventBeginPlay
  (bind _asbp_player (Utilities|Casting|CastToBP_Player (Game|Player|GetPlayerPawn 0)))
  (Variables|Default|SetPlayer _asbp_player))

(event Collision|EventActorBeginOverlap
  (params (OtherActor :type Actor%20Object%20Reference)))

(event EventTick
  (params (DeltaSeconds :type Float%20%28single-precision%29))
  (bind _player (Variables|Default|GetPlayer))
  (bind _projectilemovement (Variables|Default|GetProjectileMovement))
  (bind _forwardspeed (Variables|/Game/InfiniteMatrix/Blueprints/BP_Player.BP_Player_C|GetForwardSpeed _player))
  (bind _output_get (Variables|Default|SetElapsedTime (* (+ (Variables|Default|GetElapsedTime) DeltaSeconds) 1.05)))
  (Variables|/Script/Engine.ProjectileMovementComponent|SetInitialSpeed _projectilemovement (* _forwardspeed 1.1))
  (Variables|/Script/Engine.ProjectileMovementComponent|SetMaxSpeed _projectilemovement (* _forwardspeed 5.0))
  (if (>= _output_get 3.0)
    (Actor|DestroyActor)))

(fn ConstructionScript)