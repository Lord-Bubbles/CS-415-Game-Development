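; BP_Enemy is a hostile actor that the player can shoot for points or collide with and get hit.
; A projectile entering HitZone adds score to its owning player, updates the score widget and destroys both actors.
; A player entering HitZone triggers ProcessHit, destroys the enemy and, unless dead, shows a hurt overlay.
; A player entering PassZone simply removes the enemy.
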(event OnComponentBeginOverlap(PassZone)
  (params (OverlappedComponent :type Primitive%20Component%20Object%20Reference) (OtherActor :type Actor%20Object%20Reference) (OtherComp :type Primitive%20Component%20Object%20Reference) (OtherBodyIndex :type Integer) (bFromSweep :type Boolean) (SweepResult :type Hit%20Result%20Structure%20%28by%20ref%29))
  (Utilities|Casting|CastToBP_Player OtherActor)
  (Actor|DestroyActor))

(event OnComponentBeginOverlap(HitZone)
  (params (OverlappedComponent :type Primitive%20Component%20Object%20Reference) (OtherActor :type Actor%20Object%20Reference) (OtherComp :type Primitive%20Component%20Object%20Reference) (OtherBodyIndex :type Integer) (bFromSweep :type Boolean) (SweepResult :type Hit%20Result%20Structure%20%28by%20ref%29))
  (Utilities|FlowControl|Sequence
    (:then_0
      (bind _asbp_projectile (Utilities|Casting|CastToBP_Projectile OtherActor))
      (bind _output_get (Variables|/Game/InfiniteMatrix/Blueprints/BP_Player.BP_Player_C|SetScore (Variables|/Game/InfiniteMatrix/Blueprints/BP_Projectile.BP_Projectile_C|GetPlayer _asbp_projectile) (+ (Variables|/Game/InfiniteMatrix/Blueprints/BP_Player.BP_Player_C|GetScore (Variables|/Game/InfiniteMatrix/Blueprints/BP_Projectile.BP_Projectile_C|GetPlayer _asbp_projectile)) 2)))
      (Variables|/Game/InfiniteMatrix/UI/WBP_Score.WBP_Score_C|SetScoreValue (Variables|/Game/InfiniteMatrix/Blueprints/BP_Player.BP_Player_C|GetScoreWidget (Variables|/Game/InfiniteMatrix/Blueprints/BP_Projectile.BP_Projectile_C|GetPlayer _asbp_projectile)) _output_get)
      (Actor|DestroyActor)
      (Actor|DestroyActor _asbp_projectile))
    (:then_1
      (bind _asbp_player (Utilities|Casting|CastToBP_Player OtherActor))
      (Default|ProcessHit _asbp_player false)
      (Actor|DestroyActor)
      (if (not (Variables|/Game/InfiniteMatrix/Blueprints/BP_Player.BP_Player_C|GetIsDead _asbp_player))
        (bind _returnvalue (UserInterface|CreateWidget "/Game/InfiniteMatrix/UI/WBP_Hurt.WBP_Hurt_C"))
        (UserInterface|Viewport|AddtoViewport _returnvalue 0)))))

(event EventBeginPlay)

(event Collision|EventActorBeginOverlap
  (params (OtherActor :type Actor%20Object%20Reference)))

(event EventTick
  (params (DeltaSeconds :type Float%20%28single-precision%29)))

(fn ConstructionScript)