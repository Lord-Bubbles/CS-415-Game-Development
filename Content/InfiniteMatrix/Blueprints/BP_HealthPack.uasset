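; BP_HealthPack is a spinning health pickup that reacts to BP_Player.
; Tick yaws the pack and polls the player's health, swapping both cube materials between the standard look and a green one when health is low.
; Player overlap with TriggerZone calls ProcessHit(true) on the player and destroys the pack, while overlap with PassZone destroys it without that call.
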(event OnComponentBeginOverlap(TriggerZone)
  (params (OverlappedComponent :type Primitive%20Component%20Object%20Reference) (OtherActor :type Actor%20Object%20Reference) (OtherComp :type Primitive%20Component%20Object%20Reference) (OtherBodyIndex :type Integer) (bFromSweep :type Boolean) (SweepResult :type Hit%20Result%20Structure%20%28by%20ref%29))
  (Utilities|FlowControl|Sequence
    (:then_0
      (bind _asbp_player (Utilities|Casting|CastToBP_Player OtherActor))
      (Default|ProcessHit _asbp_player true)
      (Actor|DestroyActor))))

(event OnComponentBeginOverlap(PassZone)
  (params (OverlappedComponent :type Primitive%20Component%20Object%20Reference) (OtherActor :type Actor%20Object%20Reference) (OtherComp :type Primitive%20Component%20Object%20Reference) (OtherBodyIndex :type Integer) (bFromSweep :type Boolean) (SweepResult :type Hit%20Result%20Structure%20%28by%20ref%29))
  (Utilities|Casting|CastToBP_Player OtherActor)
  (Actor|DestroyActor))

(event EventBeginPlay)

(event Collision|EventActorBeginOverlap
  (params (OtherActor :type Actor%20Object%20Reference)))

(event EventTick
  (params (DeltaSeconds :type Float%20%28single-precision%29))
  (Transformation|AddLocalRotation (Variables|Default|GetHealthPack) (Math|Rotator|MakeRotator 0.0 0.0 (* DeltaSeconds (Variables|Default|GetRotateSpeed))) false false)
  (bind _asbp_player (Utilities|Casting|CastToBP_Player (Game|Player|GetPlayerPawn 0)))
  (Utilities|FlowControl|Sequence
    (:then_0
      (if (<= (Variables|/Game/InfiniteMatrix/Blueprints/BP_Player.BP_Player_C|GetHealth _asbp_player) 1e+02)
        (Rendering|Material|SetMaterial (Variables|Default|GetCube1) 0 "/Game/InfiniteMatrix/Materials/MI_HealthPack.MI_HealthPack")
        (Rendering|Material|SetMaterial (Variables|Default|GetCube) 0 "/Game/InfiniteMatrix/Materials/MI_HealthPack.MI_HealthPack")))
    (:then_1
      (if (< (Variables|/Game/InfiniteMatrix/Blueprints/BP_Player.BP_Player_C|GetHealth _asbp_player) 3e+01)
        (Rendering|Material|SetMaterial (Variables|Default|GetCube1) 0 "/Game/InfiniteMatrix/Materials/MI_HealthPackGreen.MI_HealthPackGreen")
        (Rendering|Material|SetMaterial (Variables|Default|GetCube) 0 "/Game/InfiniteMatrix/Materials/MI_HealthPackGreen.MI_HealthPackGreen")))))

(fn ConstructionScript)